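; BP_TCFBuilding_Base is a building Blueprint that currently drives and logs construction as a test loop.
; On BeginPlay it binds the progress and completion events, then starts a looping timer that adds fixed construction work, crediting the BP_Squad_Worker returned by GetActorOfClass.
; The event handlers print the new progress and the building's completion source; the timer is never cleared here.
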(event Custom|OnConstructionProgressChanged_Event
  (params (Building :type TCF%20Building%20Actor%20Object%20Reference) (OldProgress :type Float%20%28single-precision%29) (NewProgress :type Float%20%28single-precision%29))
  (Development|PrintString (Utilities|String|ToString(Float) NewProgress)))

(event Custom|OnConstructionCompleted_Event
  (params (Building :type TCF%20Building%20Actor%20Object%20Reference) (CompletionSource :type Actor%20Object%20Reference))
  (Development|PrintText (Utilities|Text|FormatText "{1} completed by {2}" Building CompletionSource)))

(event Custom|CustomEvent
  (bind _returnvalue (Actor|GetActorOfClass "/Game/Blueprints/Squads/BP_Squad_Worker.BP_Squad_Worker_C"))
  (Class|TCFBuildingActor|AddConstructionWork 25.0 _returnvalue))

(event EventBeginPlay
  (EventDispatchers|AssignOnConstructionProgressChanged (delegate Custom|OnConstructionProgressChanged_Event))
  (EventDispatchers|AssignOnConstructionCompleted (delegate Custom|OnConstructionCompleted_Event))
  (Utilities|Time|SetTimerbyEvent (delegate Custom|CustomEvent) 3.0 true))

(fn ConstructionScript)