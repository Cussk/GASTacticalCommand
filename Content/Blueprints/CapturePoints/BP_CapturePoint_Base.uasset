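; BP_CapturePoint_Base is a base capture point actor that shows on-screen debug feedback for its capture status.
; On BeginPlay it binds to the progress, state and owner change delegates of its CapturePointComponent.
; The handlers only print color-coded debug text: progress against threshold, the new state, and the new owner's ID.
; The Blueprint itself contains no capture logic.
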(event Custom|OnCaptureProgressChanged_Event
  (params (CaptureProgress :type Float%20%28single-precision%29) (CaptureThreshold :type Float%20%28single-precision%29))
  (Development|PrintText (Utilities|Text|FormatText "{1}/{2}" CaptureProgress CaptureThreshold) true true "(R=0.000000,G=1.000000,B=0.000000,A=1.000000)" 0.1))

(event Custom|OnCaptureStateChanged_Event
  (params (NewState :type ETCFCapturePointState%20Enum :default "Neutral"))
  (Development|PrintString (Utilities|String|EnumtoString NewState) true true "(R=1.000000,G=0.756185,B=0.002464,A=1.000000)"))

(event Custom|OnCaptureOwnerChanged_Event
  (params (NewOwnerAffiliation :type TCF%20Affiliation%20Data%20Structure) (NewOwnerSide :type TCF%20Capture%20Side%20Key%20Structure))
  (Development|PrintString (Utilities|String|ToString(Integer) (.ownerid NewOwnerAffiliation)) true true "(R=1.000000,G=0.000000,B=0.000000,A=1.000000)"))

(event EventBeginPlay
  (EventDispatchers|AssignOnCaptureProgressChanged (Variables|Default|GetCapturePointComponent) (delegate Custom|OnCaptureProgressChanged_Event))
  (EventDispatchers|AssignOnCaptureStateChanged (Variables|Default|GetCapturePointComponent) (delegate Custom|OnCaptureStateChanged_Event))
  (EventDispatchers|AssignOnCaptureOwnerChanged (Variables|Default|GetCapturePointComponent) (delegate Custom|OnCaptureOwnerChanged_Event)))

(event Collision|EventActorBeginOverlap
  (params (OtherActor :type Actor%20Object%20Reference)))

(event EventTick
  (params (DeltaSeconds :type Float%20%28single-precision%29)))

(fn ConstructionScript)