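; BP_TCFPlayerController is a player controller that binds hotkeys to RTS orders and building placement.
; Number keys start order targeting on the RTSOrderTargetingComponent with Rally, Fortify Position, Suppressive Fire or Tactical Retreat order data assets.
; The B key starts placement of a Resource Dropoff construct through the RTSBuildingPlacementComponent.
; Keys are hardwired input events, and the Blueprint only forwards data assets to those components, with no other logic.
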(event EventBeginPlay)

(event EventTick
  (params (DeltaSeconds :type Float%20%28single-precision%29)))

(event Input|KeyboardEvents|2
  (params (Key :type Key%20Structure :default "None"))
  (:Pressed
    (Class|TCFRTSOrderTargetingComponent|BeginOrderTargeting (Variables|Default|GetRTSOrderTargetingComponent) "/Game/Data/Orders/DA_Order_FortifyPosition.DA_Order_FortifyPosition")))

(event Input|KeyboardEvents|4
  (params (Key :type Key%20Structure :default "None"))
  (:Pressed
    (Class|TCFRTSOrderTargetingComponent|BeginOrderTargeting (Variables|Default|GetRTSOrderTargetingComponent) "/Game/Data/Orders/DA_Order_TacticalRetreat.DA_Order_TacticalRetreat")))

(event Input|KeyboardEvents|1
  (params (Key :type Key%20Structure :default "None"))
  (:Pressed
    (Class|TCFRTSOrderTargetingComponent|BeginOrderTargeting (Variables|Default|GetRTSOrderTargetingComponent) "/Game/Data/Orders/DA_Order_Rally.DA_Order_Rally")))

(event Input|KeyboardEvents|3
  (params (Key :type Key%20Structure :default "None"))
  (:Pressed
    (Class|TCFRTSOrderTargetingComponent|BeginOrderTargeting (Variables|Default|GetRTSOrderTargetingComponent) "/Game/Data/Orders/DA_Order_SuppressiveFire.DA_Order_SuppressiveFire")))

(event Input|KeyboardEvents|B
  (params (Key :type Key%20Structure :default "None"))
  (:Pressed
    (Class|TCFRTSBuildingPlacementComponent|BeginBuildingPlacement (Variables|Default|GetRTSBuildingPlacementComponent) "/Game/Data/Buildings/Construction/DA_Construct_ResourceDropoff.DA_Construct_ResourceDropoff")))

(fn ConstructionScript)