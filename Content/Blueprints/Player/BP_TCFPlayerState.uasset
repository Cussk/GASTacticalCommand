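; BP_TCFPlayerState is a player state Blueprint that prints the player's resource bank balances as debug text.
; On BeginPlay it binds to the PlayerResourceBankComponent's amount-changed event, then prints every current balance in green.
; Each later change prints the resource's gameplay tag name and its new amount.
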(event Custom|OnResourceAmountChanged_Event
  (params (ResourceType :type Gameplay%20Tag%20Structure) (OldAmount :type Integer) (NewAmount :type Integer))
  (Development|PrintText (Utilities|Text|FormatText "{1} : {2}" (GameplayTags|GetTagName ResourceType) NewAmount) true true "(R=0.000000,G=0.660000,B=1.000000,A=1.000000)" 5.0))

(event EventBeginPlay
  (bind _playerresourcebankcomponent (Variables|Default|GetPlayerResourceBankComponent))
  (EventDispatchers|AssignOnResourceAmountChanged _playerresourcebankcomponent (delegate Custom|OnResourceAmountChanged_Event))
  (bind (_keypin _valuepin) (Utilities|Map|ForEachLoop(Map) (Class|TCFPlayerResourceBankComponent|GetResourceBalances _playerresourcebankcomponent))
    (:then
      (Development|PrintText (Utilities|Text|FormatText "{1} : {2}" (GameplayTags|GetTagName _keypin) _valuepin) true true "(R=0.241586,G=1.000000,B=0.000000,A=1.000000)" 5.0))))

(fn ConstructionScript)